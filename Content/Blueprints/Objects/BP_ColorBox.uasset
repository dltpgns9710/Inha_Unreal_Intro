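; BP_ColorBox is a box actor that takes a random color, re-rolled whenever a BaseCharacter enters its trigger.
; BeginPlay gives the cube a dynamic material instance and applies RandomColor, which only the server randomizes.
; The RepNotify on RandomColor pushes each new value to the material's Color parameter, keeping the color synced across the network.
; If the material instance is not yet valid, the notify just prints a debug string.
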(event OnComponentBeginOverlap(Box)
  (params (OverlappedComponent :type Primitive%20Component%20Object%20Reference) (OtherActor :type Actor%20Object%20Reference) (OtherComp :type Primitive%20Component%20Object%20Reference) (OtherBodyIndex :type Integer) (bFromSweep :type Boolean) (SweepResult :type Hit%20Result%20Structure%20%28by%20ref%29))
  (Networking|SwitchHasAuthority
    (:Authority
      (Utilities|Casting|CastToBaseCharacter OtherActor)
      (Variables|Default|SetRandomColor (Math|Color|MakeColor (Math|Random|RandomFloat) (Math|Random|RandomFloat) (Math|Random|RandomFloat))))))

(event EventBeginPlay
  (bind _returnvalue (Rendering|Material|CreateDynamicMaterialInstance (Variables|Default|GetCube) 0 "/Game/Blueprints/Objects/Material/MI_ColorBox_Base.MI_ColorBox_Base" "None" :!class /Script/Engine.PrimitiveComponent))
  (bind _output_get (Variables|Default|SetMIDColor _returnvalue))
  (Rendering|Material|SetMaterial (Variables|Default|GetCube) 0 _output_get)
  (Networking|SwitchHasAuthority
    (:Authority
      (Variables|Default|SetRandomColor (Math|Color|MakeColor (Math|Random|RandomFloat) (Math|Random|RandomFloat) (Math|Random|RandomFloat))))
    (:Remote
      _))
  (Rendering|Material|SetVectorParameterValue (Variables|Default|GetMIDColor) "Color" (Variables|Default|GetRandomColor) :!class /Script/Engine.MaterialInstanceDynamic))

(event Collision|EventActorBeginOverlap
  (params (OtherActor :type Actor%20Object%20Reference)))

(event EventTick
  (params (DeltaSeconds :type Float%20%28single-precision%29)))

(fn ConstructionScript)

(fn OnRepRandomColor
  (bind _midcolor (Variables|Default|GetMIDColor))
  (Utilities|IsValid _midcolor
    (:Is%20Valid
      (Rendering|Material|SetVectorParameterValue _midcolor "Color" (Variables|Default|GetRandomColor) :!class /Script/Engine.MaterialInstanceDynamic))
    (:Is%20Not%20Valid
      (Development|PrintString "Hello"))))