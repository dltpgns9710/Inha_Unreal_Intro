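; BP_Door is a cooperative door that is destroyed once every player has interacted with it.
; Box overlap makes the player its owner, and OnInteract records each unique owner, comparing the count to the game mode's PlayerCount.
; Until all have interacted, each new player shifts DoorColor by a fixed amount, and its RepNotify applies it to the cube's dynamic material created on BeginPlay.
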(event OnComponentBeginOverlap(Box)
  (params (OverlappedComponent :type Primitive%20Component%20Object%20Reference) (OtherActor :type Actor%20Object%20Reference) (OtherComp :type Primitive%20Component%20Object%20Reference) (OtherBodyIndex :type Integer) (bFromSweep :type Boolean) (SweepResult :type Hit%20Result%20Structure%20%28by%20ref%29))
  (Utilities|Casting|CastToBP_Player OtherActor)
  (Actor|SetOwner OtherActor))

(event Custom|OnInteract
  (bind _asbp_player (Utilities|Casting|CastToBP_Player (Components|GetOwner)))
  (if (not (Utilities|Set|Contains (Variables|Default|GetInteractPlayers) _asbp_player))
    (Utilities|Set|Add (Variables|Default|GetInteractPlayers) _asbp_player)
    (bind _asbp_base_game_mode (Utilities|Casting|CastToBP_BaseGameMode (Game|GetGameMode)))
    (if (== (Variables|/Game/Blueprints/GameModes/BP_BaseGameMode.BP_BaseGameMode_C|GetPlayerCount _asbp_base_game_mode) (Utilities|Set|Length (Variables|Default|GetInteractPlayers)))
      (Actor|DestroyActor)
      (else
        (bind _returnvalue (Rendering|Material|GetVectorParameterValue (Variables|Default|GetMIDColor) "Color" :!class /Script/Engine.MaterialInstanceDynamic))
        (Variables|Default|SetDoorColor (Math|Color|MakeColor (+ (.R (Math|Color|BreakColor _returnvalue)) (Variables|Default|Getamout)) (+ (.G (Math|Color|BreakColor _returnvalue)) (Variables|Default|Getamout)) (+ (.B (Math|Color|BreakColor _returnvalue)) (Variables|Default|Getamout)) (.A (Math|Color|BreakColor _returnvalue))))))))

(event EventBeginPlay
  (bind _returnvalue (Rendering|Material|CreateDynamicMaterialInstance (Variables|Default|GetCube) 0 "/Game/Blueprints/Objects/Material/MI_ColorBox_Base.MI_ColorBox_Base" "None" :!class /Script/Engine.PrimitiveComponent))
  (bind _output_get (Variables|Default|SetMIDColor _returnvalue))
  (Rendering|Material|SetMaterial (Variables|Default|GetCube) 0 _output_get))

(event Collision|EventActorBeginOverlap
  (params (OtherActor :type Actor%20Object%20Reference)))

(event EventTick
  (params (DeltaSeconds :type Float%20%28single-precision%29)))

(fn ConstructionScript)

(fn OnRepDoorColor
  (bind _midcolor (Variables|Default|GetMIDColor))
  (Utilities|IsValid _midcolor
    (:Is%20Valid
      (Rendering|Material|SetVectorParameterValue _midcolor "Color" (Variables|Default|GetDoorColor) :!class /Script/Engine.MaterialInstanceDynamic))))