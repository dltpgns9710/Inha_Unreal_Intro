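; BP_InteractDoor is a door actor that swings open and closed when its Interact event fires.
; Each interaction flips DoorOpen and stops the DoorAnimation timeline, then plays it from the start or reverses it from the end, so an interrupted swing jumps to an endpoint.
; The timeline's RotationZ track drives the static mesh's relative yaw.
; CanInteract always returns false, regardless of the instigating character.
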(event EventBeginPlay)

(event Collision|EventActorBeginOverlap
  (params (OtherActor :type Actor%20Object%20Reference)))

(event EventTick
  (params (DeltaSeconds :type Float%20%28single-precision%29)))

(event EventInteract
  (params (CharacterInstigator :type Base%20Character%20Object%20Reference))
  (Variables|Default|SetDoorOpen (not (Variables|Default|GetDoorOpen)))
  (Audio|Components|Audio|Stop (Variables|Default|GetDoorAnimation))
  (if (Variables|Default|GetDoorOpen)
    (bind _rotationz (Timeline|DoorAnimation PlayFromStart)
      (:Update
        (Transformation|SetRelativeRotation (Variables|Default|GetStaticMesh) (Math|Rotator|MakeRotator 0.0 0.0 _rotationz) false false)))
    (else
      (Timeline|DoorAnimation ReverseFromEnd))))

(fn ConstructionScript)

(fn CanInteract
  (params (CharacterInstigator :type Base%20Character%20Object%20Reference))
  (return false))