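; Base game mode that counts connected players, hands out spawn points and assigns player skins.
; PostLogin and OnLogout adjust the player count.
; ChoosePlayerStart returns the first PlayerStart not tagged "Used" and tags it, so each start is given out only once.
; On player restart, the controlled BP_Player receives the next material from the skin array via an incrementing index that never wraps or resets here.
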(event EventPostLogin
  (params (NewPlayer :type Player%20Controller%20Object%20Reference))
  (Variables|Default|SetPlayerCount (+ (Variables|Default|GetPlayerCount) 1)))

(event EventOnLogout
  (params (ExitingController :type Controller%20Object%20Reference))
  (Variables|Default|SetPlayerCount (- (Variables|Default|GetPlayerCount) 1)))

(event EventOnRestartPlayer
  (params (NewPlayer :type Controller%20Object%20Reference))
  (bind _asbp_player (Utilities|Casting|CastToBP_Player (Pawn|GetControlledPawn NewPlayer)))
  (Variables|/Game/Blueprints/Character/Player/BP_Player.BP_Player_C|SetSkinMaterial _asbp_player (Utilities|Array|Get(acopy) (Variables|Default|GetSkinMaterials) (Variables|Default|GetSkinCount)))
  (Variables|Default|SetSkinCount (+ (Variables|Default|GetSkinCount) 1)))

(fn ConstructionScript)

(fn ChoosePlayerStart
  (params (Player :type Controller%20Object%20Reference))
  (bind _outactors (Actor|GetAllActorsOfClass "/Script/Engine.PlayerStart"))
  (for _array_element _outactors
    (if (!= "Used" (Variables|/Script/Engine.PlayerStart|GetPlayerStartTag _array_element))
      (Variables|/Script/Engine.PlayerStart|SetPlayerStartTag _array_element "Used")
      (return _array_element))))