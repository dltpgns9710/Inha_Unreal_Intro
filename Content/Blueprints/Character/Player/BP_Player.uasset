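; Player character Blueprint that handles weapon and HP notifications, points, the game-over screen and door interaction.
; BeginPlay broadcasts weapon and HP state, then binds game-over to show WBP_GameOver with the cursor and weapon changes to rebroadcast the type.
; Outside dedicated servers, a timeline drives a Niagara spawn-in effect and dynamic materials' SpawnAge together.
; F interacts with the BP_Door found by GetActorOfClass, and OnRep functions refresh points text and skin material.
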(event Custom|커스텀이벤트
  (bind _returnvalue (CallFunction|GetWeponTypebyCompponent))
  (Default|CallOnWeaponChanged _returnvalue))

(event Custom|커스텀이벤트_0
  (bind _returnvalue (Game|GetPlayerController 0))
  (Variables|/Script/Engine.PlayerController|SetbShowMouseCursor _returnvalue true)
  (bind _returnvalue_2 (UserInterface|CreateWidget "/Game/Blueprints/Widget/WBP_GameOver.WBP_GameOver_C" _returnvalue))
  (UserInterface|Viewport|AddtoViewport _returnvalue_2 0))

(event EventBeginPlay
  (Utilities|FlowControl|Sequence
    (:then_1
      (bind _returnvalue (CallFunction|GetWeponTypebyCompponent))
      (Default|CallOnWeaponChanged _returnvalue)
      (CallFunction|CalcHP)
      (Utilities|FlowControl|Sequence
        (:then_0
          (EventDispatchers|BindEventtoOnGameOver (delegate Custom|커스텀이벤트_0)))
        (:then_1
          (EventDispatchers|BindEventtoOnWeaponChange (delegate Custom|커스텀이벤트)))))
    (:then_2
      (if (not (Networking|IsDedicatedServer))
        (CallFunction|CreateDynamicMaterials)
        (bind _returnvalue_2 (Niagara|SpawnSystemAttached "/Game/Assets/Effects/Particles/Environmental/NS_CharacterSpawnIn2.NS_CharacterSpawnIn2" (Variables|Character|GetMesh) "None" "0, 0, 0" "0, 0, 0" "KeepRelativeOffset" false))
        (Variables|Default|SetSpawnEffect _returnvalue_2)
        (Components|Timeline|SetPlayRate (Variables|Default|GetSpawn) (/ 1.0 (Variables|Default|GetSpawn%20Time)))
        (Niagara|SetNiagaraVariable(Float) (Variables|Default|GetSpawnEffect) "SpawnTimeLength" (Variables|Default|GetSpawn%20Time))
        (bind _spawntimeline (Timeline|Spawn PlayFromStart)
          (:Update
            (Niagara|SetNiagaraVariable(Float) (Variables|Default|GetSpawnEffect) "SpawnTimeline" _spawntimeline)
            (for _array_element (Variables|Default|GetMaterials)
              (Rendering|Material|SetScalarParameterValue _array_element "SpawnAge" _spawntimeline :!class /Script/Engine.MaterialInstanceDynamic))))))))

(event EventAddPoint
  (params (Point :type Integer))
  (Variables|Default|SetPoints (+ Point (Variables|Default|GetPoints))))

(event Input|KeyboardEvents|F
  (params (Key :type Key%20Structure :default "None"))
  (:Pressed
    (bind _returnvalue (Actor|GetActorOfClass "/Game/Blueprints/Objects/BP_Door.BP_Door_C"))
    (Default|Interact _returnvalue)))

(fn ConstructionScript)

(fn CalcHP
  (Default|CallOnHPChanged (/ (Variables|Default|GetHp) (Variables|Default|GetInitHp)) (Utilities|String|Append (Utilities|String|ToString(Float) (Variables|Default|GetHp)) "/" (Utilities|String|ToString(Float) (Variables|Default|GetInitHp)))))

(fn GetWeponTypebyCompponent
  (Utilities|IsValid (Variables|Default|GetCasted%20Player%20Attack%20Component)
    (:Is%20Valid
      (bind _returnvalue (Class|PlayerAttackComponent|GetWeaponType (Variables|Default|GetCasted%20Player%20Attack%20Component) :!label _label)))
    (:Is%20Not%20Valid
      (bind _asplayer_attack_component (Utilities|Casting|CastToPlayerAttackComponent (Variables|Default|GetPlayerAttackComponent))
        (:then
          (Variables|Default|SetCasted%20Player%20Attack%20Component _asplayer_attack_component)
          (goto _label))
        (:CastFailed
          _))))
  (return _returnvalue))

(fn CreateDynamicMaterials
  (Utilities|Array|Clear (Variables|Default|GetMaterials))
  (for (_array_element _array_index) (Rendering|Material|GetMaterials (Variables|Character|GetMesh))
    (bind _returnvalue (Rendering|Material|CreateDynamicMaterialInstance _array_element "None" "None" :!class /Script/Engine.KismetMaterialLibrary))
    (Utilities|Array|Add (Variables|Default|GetMaterials) _returnvalue)
    (Rendering|Material|SetMaterial (Variables|Character|GetMesh) _array_index _returnvalue)))

(fn OnRepPoints
  (Rendering|Components|TextRender|SetText (Variables|Default|GetPoint) (Utilities|Text|ToText(Integer) (Variables|Default|GetPoints))))

(fn OnRepSkinMaterial
  (Rendering|Material|SetMaterial (Variables|Character|GetMesh) 0 (Variables|Default|GetSkinMaterial)))