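; BP_PointSpawner is an actor that periodically spawns random objects within a box area.
; On BeginPlay, only the server authority starts a looping one-second timer that calls Spawn.
; Spawn picks a random class from the SpawnObjects array and places it at a random point inside the SpawnArea box's scaled extent around the actor's location.
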(event Custom|SpawnActor
  (CallFunction|Spawn))

(event EventBeginPlay
  (Networking|SwitchHasAuthority
    (:Authority
      (Utilities|Time|SetTimerbyEvent (delegate Custom|SpawnActor) 1.0 true))))

(event Collision|EventActorBeginOverlap
  (params (OtherActor :type Actor%20Object%20Reference)))

(event EventTick
  (params (DeltaSeconds :type Float%20%28single-precision%29)))

(fn ConstructionScript)

(fn Spawn
  (Game|SpawnActorfromClass (.OutItem (Utilities|Array|Random (Variables|Default|GetSpawnObjects))) (Math|Transform|MakeTransform (Math|Random|RandomPointinBoundingBox (Transformation|GetActorLocation) (Components|Box|GetScaledBoxExtent (Variables|Default|GetSpawnArea))) "0, 0, 0" "1.000000,1.000000,1.000000") "Undefined" "MultiplyWithRoot" 0 0))