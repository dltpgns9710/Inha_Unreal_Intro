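; Player controller that creates the local player's WBP_HUD and keeps its health, weapon, XP and level displays up to date.
; On BeginPlay it binds to BP_Player's HP and weapon change events and seeds the health display from current and initial HP.
; For local players it also binds to Inha_PlayerState's XP and level events, retrying on a short delay until the PlayerState cast succeeds.
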(event Custom|OnHPChanged_이벤트
  (params (HpRatio :type Float%20%28double-precision%29) (HpString :type String))
  (CallFunction|UpdateHUD HpRatio HpString))

(event Custom|OnXpChanged_이벤트
  (params (NewXp :type Integer))
  (Variables|/Game/Blueprints/Widget/WBP_HUD.WBP_HUD_C|SetXpString (Variables|Default|GetHUD) (Utilities|String|Append "XP : " (Utilities|String|ToString(Integer) NewXp))))

(event Custom|OnLevelChanged_이벤트
  (params (NewLevelXp :type Integer))
  (Variables|/Game/Blueprints/Widget/WBP_HUD.WBP_HUD_C|SetLevelString (Variables|Default|GetHUD) (Utilities|String|Append "Level : " (Utilities|String|ToString(Integer) NewLevelXp))))

(event Custom|OnWeaponChanged_이벤트
  (params (EquippedWeapon :type Byte))
  (Variables|/Game/Blueprints/Widget/WBP_HUD.WBP_HUD_C|SetEquippedWeapon (Variables|Default|GetHUD) (Utilities|Enum|ByteToEnumEWeaponType EquippedWeapon)))

(event EventBeginPlay
  (bind _returnvalue (Pawn|GetControlledPawn))
  (bind _playerstate (Variables|/Script/Engine.Pawn|GetPlayerState _returnvalue))
  (bind (_asinha_player_state _bsuccess) (Utilities|Casting|CastToInha_PlayerState _playerstate))
  (Utilities|FlowControl|Sequence
    (:then_0
      (if (Pawn|IsLocalPlayerController)
        (bind _returnvalue_2 (UserInterface|CreateWidget "/Game/Blueprints/Widget/WBP_HUD.WBP_HUD_C" self))
        (bind _output_get (Variables|Default|SetHUD _returnvalue_2))
        (UserInterface|Viewport|AddtoViewport _output_get 0)))
    (:then_1
      (bind _asbp_player (Utilities|Casting|CastToBP_Player (Pawn|GetControlledPawn)))
      (Variables|Default|SetCasted%20BP%20Player _asbp_player)
      (Utilities|FlowControl|Sequence
        (:then_0
          (EventDispatchers|AssignOnHPChanged (Variables|Default|GetCasted%20BP%20Player) (delegate Custom|OnHPChanged_이벤트))
          (CallFunction|InitHud))
        (:then_1
          (EventDispatchers|AssignOnWeaponChanged (Variables|Default|GetCasted%20BP%20Player) (delegate Custom|OnWeaponChanged_이벤트)))))
    (:then_2
      (if (Pawn|IsLocalPlayerController)
        (if _bsuccess :!label _label
          (Utilities|FlowControl|Sequence
            (:then_0
              (EventDispatchers|AssignOnXpChanged _asinha_player_state (delegate Custom|OnXpChanged_이벤트))
              (Variables|/Game/Blueprints/Widget/WBP_HUD.WBP_HUD_C|SetXpString (Variables|Default|GetHUD) "XP : 0"))
            (:then_1
              (EventDispatchers|AssignOnLevelChanged _asinha_player_state (delegate Custom|OnLevelChanged_이벤트))
              (Variables|/Game/Blueprints/Widget/WBP_HUD.WBP_HUD_C|SetLevelString (Variables|Default|GetHUD) "Level : 1")))
          (else
            (Utilities|FlowControl|Delay 0.2)
            (goto _label)))))))

(fn ConstructionScript)

(fn UpdateHUD
  (params (HPRatio :type Float%20%28double-precision%29) (HPString :type String))
  (Variables|/Game/Blueprints/Widget/WBP_HUD.WBP_HUD_C|SetHpRatio (Variables|Default|GetHUD) HPRatio)
  (Variables|/Game/Blueprints/Widget/WBP_HUD.WBP_HUD_C|SetHpString (Variables|Default|GetHUD) HPString))

(fn InitHud
  (bind _casted_bp_player (Variables|Default|GetCasted%20BP%20Player))
  (bind _casted_bp_player_2 (Variables|Default|GetCasted%20BP%20Player))
  (bind _hp (Variables|/Script/Inha_Intro.BaseCharacter|GetHp _casted_bp_player_2))
  (bind _inithp (Variables|/Script/Inha_Intro.BaseCharacter|GetInitHp _casted_bp_player))
  (CallFunction|UpdateHUD (/ _hp _inithp) (Utilities|String|Append (Utilities|String|ToString(Float) _hp) "/" (Utilities|String|ToString(Float) _inithp))))